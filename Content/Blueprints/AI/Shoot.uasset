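; Behavior tree task that makes an AI-controlled Character_BP aim and shoot at its target.
; On execute it sets the pawn's Aiming and Shooting flags and focuses the controller on the actor in the Target blackboard key.
; It never finishes execution itself, so it runs until aborted.
; On abort it clears both flags and the focus, then finishes the abort.
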(event `self.ReceiveExecuteAI`
  (params (OwnerController :type "AIController Object Reference") (ControlledPawn :type "Pawn Object Reference"))
  (bind _ascharacter_bp (cast `/Game/Blueprints/Character_BP` ControlledPawn))
  (set `/Game/Blueprints/Character_BP.Aiming` true _ascharacter_bp)
  (set `/Game/Blueprints/Character_BP.Shooting` true _ascharacter_bp)
  (`AIController.K2_SetFocus` OwnerController (`BTFunctionLibrary.GetBlackboardValueAsActor` (`self.Target`))))

(event `self.ReceiveAbortAI`
  (params (OwnerController :type "AIController Object Reference") (ControlledPawn :type "Pawn Object Reference"))
  (bind _ascharacter_bp (cast `/Game/Blueprints/Character_BP` ControlledPawn))
  (set `/Game/Blueprints/Character_BP.Aiming` false _ascharacter_bp)
  (set `/Game/Blueprints/Character_BP.Shooting` false _ascharacter_bp)
  (`AIController.K2_ClearFocus` OwnerController)
  (`self.FinishAbort`))