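; AI controller for guard NPCs that runs the GuardBehaviour behavior tree on the PatrolData blackboard.
; AI perception writes sensed actors without the "Enemy" tag to the enemy blackboard key and clears it when such an actor's sensing fails.
; Each tick, the controlled Character_BP's Aiming and Shooting flags mirror whether the controller has a valid focus actor, which is not set in this graph.
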(event `self.ReceiveBeginPlay`
  (bind _blackboardcomponent (`self.UseBlackboard` "/Game/Blueprints/AI/PatrolData.PatrolData"))
  (`self.RunBehaviorTree` "/Game/Blueprints/AI/GuardBehaviour.GuardBehaviour")
  (set `self.BlackboardComp` _blackboardcomponent))

(event `self.AIPerception.OnTargetPerceptionUpdated`
  (params (Actor :type "Actor Object Reference") (Stimulus :type "AIStimulus Structure"))
  (bind _enemykey (`self.Enemykey`))
  (bind _blackboardcomp (`self.BlackboardComp`))
  (if (`self.ActorHasTag` Actor "Enemy")
    _
    (elif (`.bSuccessfullySensed` (break `AIStimulus` Stimulus))
      (`BlackboardComponent.SetValueAsObject` _blackboardcomp _enemykey Actor)
      (else
        (`BlackboardComponent.ClearValue` _blackboardcomp _enemykey)))))

(event `self.ReceiveTick`
  (params (DeltaSeconds :type "Float (single-precision)"))
  (bind _returnvalue (`KismetSystemLibrary.IsValid` (`self.GetFocusActor`)))
  (bind _ascharacter_bp (cast `/Game/Blueprints/Character_BP` (`self.K2_GetPawn`)))
  (set `/Game/Blueprints/Character_BP.Aiming` _returnvalue _ascharacter_bp)
  (set `/Game/Blueprints/Character_BP.Shooting` _returnvalue _ascharacter_bp))

(fn `UserConstructionScript`)