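; NPC_AI_BP is an AI controller for guard NPCs that runs the GuardBehaviour behavior tree on the PatrolData blackboard.
; AI Perception writes sensed actors without the "Enemy" tag to the blackboard's enemy key and clears it when sensing is lost.
; Every tick it sets the possessed PatrollingGuard2's Aiming and Shooting flags according to whether the controller has a valid focus actor.
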(event `self.ReceiveBeginPlay`
  (bind _blackboardcomponent (`self.UseBlackboard` "/Game/Blueprints/PatrolData.PatrolData"))
  (`self.RunBehaviorTree` "/Game/Blueprints/GuardBehaviour.GuardBehaviour")
  (set `self.BlackboardComp` _blackboardcomponent))

(event `self.AIPerception.OnTargetPerceptionUpdated`
  (params (Actor :type "Actor Object Reference") (Stimulus :type "AIStimulus Structure"))
  (bind _enemykey (`self.Enemykey`))
  (bind _blackboardcomp (`self.BlackboardComp`))
  (if (`self.ActorHasTag` Actor "Enemy")
    _
    (elif (`.bSuccessfullySensed` (break `AIStimulus` Stimulus))
      (`BlackboardComponent.SetValueAsObject` _blackboardcomp _enemykey Actor)
      (else
        (`BlackboardComponent.ClearValue` _blackboardcomp _enemykey)))))

(event `self.ReceiveTick`
  (params (DeltaSeconds :type "Float (single-precision)"))
  (bind _aspatrolling_guard_2 (cast `/Game/AnimStarterPack/PatrollingGuard2` (`self.K2_GetPawn`)))
  (bind _output_get (set `/Game/AnimStarterPack/PatrollingGuard2.Aiming` (`KismetSystemLibrary.IsValid` (`self.GetFocusActor`)) _aspatrolling_guard_2))
  (set `/Game/AnimStarterPack/PatrollingGuard2.Shooting` _output_get _aspatrolling_guard_2))

(fn `UserConstructionScript`)